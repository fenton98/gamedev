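; Ring pickup Blueprint that extends a parent pickup and adds behavior for rings spawned as dropped.
; On BeginPlay, a dropped ring disables its inner and outer collision, enables gravity on its physics sphere and launches it at a random angle in the XZ plane.
; After a short delay collision returns, and if the sphere is still valid the ring destroys itself shortly afterward.
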(event EventBeginPlay
  (bind _force (Variables|Default|GetForce))
  (bind _direction (Variables|Default|GetDirection))
  (bind _direction_2 (Variables|Default|GetDirection))
  (bind _returnvalue (* _direction_2 -1.0))
  (bind _returnvalue_2 (Math|Random|RandomFloatinRange _returnvalue _direction))
  (|CallParentFunction)
  (if (Variables|Default|GetbDropped)
    (Collision|SetCollisionEnabled (Variables|Default|GetInnerCollision) "NoCollision")
    (Collision|SetCollisionEnabled (Variables|Default|GetOutterCollision) "NoCollision")
    (Physics|SetEnableGravity (Variables|Default|GetSphere) true)
    (Class|PrimitiveComponent|SetAllPhysicsLinearVelocity (Variables|Default|GetSphere) (Math|Vector|MakeVector (* (Math|Trig|Sin(Degrees) _returnvalue_2) _force) 0.0 (* (Math|Trig|Cos(Degrees) _returnvalue_2) _force)) false)
    (Utilities|FlowControl|Delay 1.0)
    (Collision|SetCollisionEnabled (Variables|Default|GetInnerCollision) "QueryAndPhysics")
    (Utilities|IsValid (Variables|Default|GetSphere)
      (:Is%20Valid
        (Collision|SetCollisionEnabled (Variables|Default|GetOutterCollision) "QueryAndPhysics")
        (Utilities|FlowControl|Delay 2.0)
        (Actor|DestroyActor)))))

(fn ConstructionScript
  (|CallParentFunction))