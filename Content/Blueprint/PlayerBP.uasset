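; Player character for a 2D side-scrolling platformer, with running, double and wall jumps, dashing, climbing and delayed projectile attacks.
; A line trace detects walls for launches, and timelines add squash with dust on jump and landing.
; Tick flips the sprite and picks its flipbook through a state-selection function.
; Damage removes mushroom growth or drops rings, both tracked in GameControllerBP, otherwise destroys the player; Health is unused.
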(event Custom|WallJump
  (bind _returnvalue (Transformation|GetActorForwardVector))
  ;[1 1 1] wall jump
  (bind (_outhit _returnvalue_2) (Collision|LineTraceByChannel (- (Transformation|GetActorLocation) (* _returnvalue (+ (Components|Capsule|GetScaledCapsuleRadius (Variables|Collision|GetCapsuleComponent)) 15.0))) (+ (Transformation|GetActorLocation) (* _returnvalue (+ (Components|Capsule|GetScaledCapsuleRadius (Variables|Collision|GetCapsuleComponent)) 15.0))) "TraceTypeQuery1" true 0 "None"))
  (if _returnvalue_2
    (Character|LaunchCharacter (Math|Vector|MakeVector (* (Math|Float|Sign(Float) (- (.x (Transformation|GetActorLocation)) (.x (.Location (Collision|BreakHitResult _outhit))))) 4.5e+02) 0.0 (Variables|/Script/Engine.CharacterMovementComponent|GetJumpZVelocity (Variables|Character|GetCharacterMovement))) true true)
    (CallFunction|JumpFX)
    (elif (< (Variables|Default|GetJumpCurrentCount) 2)
      (Character|Jump)
      (Variables|Default|SetJumpMaxCount (+ (Variables|Default|GetJumpCurrentCount) 1))
      (CallFunction|JumpFX))))

(event Custom|JumpFX
  (Effects|SpawnEmitteratLocation "/Game/Art/Particles/pDust.pDust" (Transformation|GetWorldLocation (Variables|Default|GetDustBox)))
  (bind _squash (Timeline|Timeline_0 PlayFromStart)
    (:Update
      (Transformation|SetActorScale3D (Math|Vector|Lerp(Vector) (Variables|Default|GetCurrentScale) "0.500000,0.500000,0.500000" _squash)))))

(event Custom|LandFX
  (Effects|SpawnEmitteratLocation "/Game/Art/Particles/pDust.pDust" (Transformation|GetWorldLocation (Variables|Default|GetDustBox)))
  (bind _squash (Timeline|Timeline_1 PlayFromStart)
    (:Update
      (Transformation|SetActorScale3D (Math|Vector|Lerp(Vector) (Variables|Default|GetCurrentScale) "0.500000,0.500000,0.500000" _squash)))))

(event Custom|UpdateAnimation
  (bind _charactermovement (Variables|Character|GetCharacterMovement))
  (bind _returnvalue (AI|Components|NavMovement|IsFalling _charactermovement))
  ;[1 1 1] Animation state machine
  (Variables|Default|SetbIsMoving (> (Math|Vector|VectorLength (Transformation|GetVelocity)) 0.0))
  (bind _outputfb (CallFunction|AnimationStateMachine (Variables|Default|GetbIsMoving) _returnvalue _returnvalue (Variables|Default|GetbIsAttacking) (Variables|Default|GetbIsClimbing)))
  (Sprite|SetFlipbook (Variables|Default|GetSprite) _outputfb))

(event Custom|FireProjectile
  ;[1 1 1] Fire
  (Game|SpawnActorfromClass "/Game/Blueprint/ProjectileBP.ProjectileBP_C" (Transformation|GetWorldTransform (Variables|Default|GetProjectileSpawn)) "AlwaysSpawn" 0 0))

(event Custom|AttackAnimation
  (Utilities|FlowControl|Sequence
    (:then_0
      (Variables|Default|SetbIsAttacking true)
      (Utilities|FlowControl|Delay 0.6)
      (CallFunction|FireProjectile))
    (:then_1
      (Utilities|FlowControl|Delay 1.0)
      (Variables|Default|SetbIsAttacking false))))

(event Custom|ClimbingEnd
  (Pawn|Components|CharacterMovement|SetMovementMode (Variables|Character|GetCharacterMovement) "MOVE_Walking" 0)
  (Variables|Default|SetbIsClimbing false)
  (Components|Timeline|SetPlayRate (Variables|Default|GetSprite) 1.0))

(event Custom|ScaleControl
  (params (bIsHealth :type Boolean))
  ;[1 1 1] Health Size Swap
  (if bIsHealth
    (if (not (Variables|/Game/Blueprint/GameControllerBP.GameControllerBP_C|GetbHasMushroom (Variables|Default|GetGameController)))
      (bind _scalelerp (Timeline|Scale Play)
        (:Update
          (Transformation|SetActorScale3D _scalelerp)
          (Variables|Default|SetCurrentScale (Variables|Default|GetIncreasedScale))
          (Variables|/Game/Blueprint/GameControllerBP.GameControllerBP_C|SetbHasMushroom (Variables|Default|GetGameController) true))))
    (else
      (Variables|Default|SetCurrentScale (Variables|Default|GetStartScale))
      (Transformation|SetActorScale3D (Variables|Default|GetStartScale))
      (Variables|/Game/Blueprint/GameControllerBP.GameControllerBP_C|SetbHasMushroom (Variables|Default|GetGameController) false))))

(event Custom|DropRing
  (for _index (range 0 (- (Variables|/Game/Blueprint/GameControllerBP.GameControllerBP_C|GetRingsCollected (Variables|Default|GetGameController)) 1))
    (Game|SpawnActorfromClass "/Game/Blueprint/PickUps/bpPickUpRing.bpPickUpRing_C" (Transformation|GetActorTransform) "Undefined" 0 true 0))
  (Variables|/Game/Blueprint/GameControllerBP.GameControllerBP_C|SetRingsCollected (Variables|Default|GetGameController) 0))

(event EventTick
  (params (DeltaSeconds :type Float%20%28single-precision%29))
  ;[1 1 1] Update
  (CallFunction|UpdateAnimation)
  (Math|Float|CompareFloat (.X (Math|Vector|BreakVector (Variables|/Script/Engine.MovementComponent|GetVelocity (Variables|Character|GetCharacterMovement)))) 0.0
    (:>
      (Transformation|SetRelativeRotation (Variables|Default|GetSprite) "0, 0, 0" false false))
    (:<
      (Transformation|SetRelativeRotation (Variables|Default|GetSprite) "0,180.000000, 0" false false))))

(event EventBeginPlay
  ;[1 1 1] Begin Play
  (bind _asgame_controller_bp (Utilities|Casting|CastToGameControllerBP (Game|GetGameMode)))
  (Variables|Default|SetGameController _asgame_controller_bp))

(event EventOnLanded
  (params (Hit :type Hit%20Result%20Structure%20%28by%20ref%29))
  ;[1 1 1] Landed
  (Variables|Default|SetJumpMaxCount 0)
  (CallFunction|LandFX))

(event Game|Damage|EventAnyDamage
  (params (Damage :type Float%20%28single-precision%29) (DamageType :type Damage%20Type%20Object%20Reference) (InstigatedBy :type Controller%20Object%20Reference) (DamageCauser :type Actor%20Object%20Reference))
  (bind _gamecontroller (Variables|Default|GetGameController))
  ;[1 1 1] Death Function
  (if (or (Variables|/Game/Blueprint/GameControllerBP.GameControllerBP_C|GetbHasMushroom _gamecontroller) (> (Variables|/Game/Blueprint/GameControllerBP.GameControllerBP_C|GetRingsCollected _gamecontroller) 0))
    (if (Variables|/Game/Blueprint/GameControllerBP.GameControllerBP_C|GetbHasMushroom (Variables|Default|GetGameController))
      (CallFunction|ScaleControl false)
      (else
        (CallFunction|DropRing)))
    (else
      (Effects|SpawnEmitteratLocation "/Game/Art/Particles/pDust.pDust" "0, 0, 0")
      (Actor|DestroyActor))))

(event Input|ActionEvents|InputActionJump
  (params (Key :type Key%20Structure :default "None"))
  ;[1 1 1] Jumping section
  (:Pressed
    (Character|Jump)
    (if (AI|Components|NavMovement|IsFalling (Variables|Character|GetCharacterMovement))
      (CallFunction|WallJump)
      (else
        (Character|Jump)
        (Variables|Default|SetJumpMaxCount (+ (Variables|Default|GetJumpCurrentCount) 1))
        (CallFunction|JumpFX))))
  (:Released
    (Character|StopJumping)))

(event Input|ActionEvents|InputActionDash
  (params (Key :type Key%20Structure :default "None"))
  (bind _returnvalue (Transformation|GetVelocity))
  ;[1 1 1] Dash
  (:Pressed
    (if (Class|KismetMathLibrary|NotEqualExactlyVectorVector _returnvalue "0, 0, 0")
      (if (AI|Components|NavMovement|IsFalling (Variables|Character|GetCharacterMovement))
        (Character|LaunchCharacter (* (+ _returnvalue "0, 0, 0") "1.500000,1.500000,1.500000") true true)
        (else
          (Character|LaunchCharacter (* (+ _returnvalue "0, 0,1.000000") "1.500000,1.500000,250.000000") true true))))))

(event Input|ActionEvents|InputActionFire
  (params (Key :type Key%20Structure :default "None"))
  ;[1 1 1] Fire
  (:Pressed
    (if (not (Variables|Default|GetbIsAttacking))
      (CallFunction|AttackAnimation))))

(event Input|AxisEvents|InputAxisRight
  (params (AxisValue :type Float%20%28single-precision%29))
  (Pawn|Input|AddMovementInput "1.000000, 0, 0" AxisValue false))

(event Input|AxisEvents|InputAxisMoveUp
  (params (AxisValue :type Float%20%28single-precision%29))
  (if (Variables|Default|GetbCanClimb)
    (if (Math|Float|InRange(Float) AxisValue -0.1 0.1)
      (Components|Timeline|SetPlayRate (Variables|Default|GetSprite) 0.0)
      (else
        (Variables|Default|SetbIsClimbing true)
        (Components|Timeline|SetPlayRate (Variables|Default|GetSprite) 1.0)
        (Pawn|Components|CharacterMovement|SetMovementMode (Variables|Character|GetCharacterMovement) "MOVE_Flying" 0)
        (Pawn|Input|AddMovementInput "0, 0,0.500000" AxisValue false)))))

(fn ConstructionScript
  (Variables|/Script/Engine.CharacterMovementComponent|SetJumpZVelocity (Variables|Character|GetCharacterMovement) 2e+02)
  (Variables|Default|SetJumpMaxHoldTime 0.3)
  (Variables|Default|SetJumpCount 0)
  (bind _output_get (Variables|Default|SetStartScale (Transformation|GetActorScale3D)))
  (Variables|Default|SetCurrentScale _output_get)
  (Variables|Default|SetHealth (Variables|Default|GetMaxHealth)))

(fn AnimationStateMachine
  (params (bIsMoving :type Boolean) (bIsFalling :type Boolean) (bIsDashing :type Boolean) (bIsAttacking :type Boolean) (bIsClimbing :type Boolean))
  (if bIsClimbing
    (LocalVariables|SetAnimationState "NewEnumerator5")
    (elif bIsDashing
      (LocalVariables|SetAnimationState "NewEnumerator3")
      (elif bIsAttacking
        (LocalVariables|SetAnimationState "NewEnumerator4")
        (elif bIsFalling
          (LocalVariables|SetAnimationState "NewEnumerator2")
          (elif bIsMoving
            (LocalVariables|SetAnimationState "NewEnumerator1")
            (else
              (LocalVariables|SetAnimationState "NewEnumerator0")))))))
  (return (Utilities|Select :Index (LocalVariables|GetAnimationState) :NewEnumerator0 "/Game/Art/Flipbooks/fAlienIdle.fAlienIdle" :NewEnumerator1 "/Game/Art/Flipbooks/fAlienRun.fAlienRun" :NewEnumerator2 "/Game/Art/Flipbooks/fAlienJump.fAlienJump" :NewEnumerator3 "/Game/Art/Flipbooks/fAlienJump.fAlienJump" :NewEnumerator4 "/Game/Art/Flipbooks/fAlienAttack.fAlienAttack" :NewEnumerator5 "/Game/Art/Flipbooks/fAlienWalk.fAlienWalk")))