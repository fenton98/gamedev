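; Arrow trap or launcher actor that spawns a BpArrow every second while being moved vertically.
; On BeginPlay it records its start location, starts a looping timer that calls Fire, and plays the Movement timeline.
; The timeline lerps the actor between its start location and a point 100 units above it.
; Fire spawns each arrow at the SpawnPoint component's world transform.
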(event Custom|Fire
  (Game|SpawnActorfromClass "/Game/Blueprint/bpArrow.bpArrow_C" (Transformation|GetWorldTransform (Variables|Default|GetSpawnPoint)) "Undefined" 0 0))

(event EventBeginPlay
  (Variables|Default|SetStartPos (Transformation|GetActorLocation))
  (Utilities|Time|SetTimerbyFunctionName 0 "Fire" 1.0 true)
  (bind _move (Timeline|Movement PlayFromStart)
    (:Update
      (Transformation|SetActorLocation (Math|Vector|Lerp(Vector) (Variables|Default|GetStartPos) (Math|Vector|MakeVector (.x (Variables|Default|GetStartPos)) (.y (Variables|Default|GetStartPos)) (+ (.z (Variables|Default|GetStartPos)) 1e+02)) _move) false false))))

(fn ConstructionScript)